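; BP_HealVolume is a debug volume that periodically applies a gameplay effect, presumably healing, to characters inside it.
; A looping timer started on BeginPlay fires every few seconds and, on the server only, gathers actors overlapping EffectCollision.
; Each living NDDCharacter with an Ability System Component applies the configured GameplayEffectClass to itself through GAS.
; The tick event is named OnDamageTick, so the actual result depends on that effect class.
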(event `self.ReceiveBeginPlay`
  (`KismetSystemLibrary.K2_SetTimerDelegate` (delegate `OnDamageTick`) 2.5 true))

(event `OnDamageTick`
  (`/Engine/EditorBlueprintResources/ActorMacros.Switch Has Authority`
    (:`Authority`
      (for _array_element (`PrimitiveComponent.GetOverlappingActors` (`self.EffectCollision`) null)
        (bind _asnddcharacter (cast `NDDCharacter` _array_element))
        (bind _returnvalue (`AbilitySystemBlueprintLibrary.GetAbilitySystemComponent` _asnddcharacter))
        (if (and (`NDDCharacter.IsAlive` _asnddcharacter) (`KismetSystemLibrary.IsValid` _returnvalue))
          (`AbilitySystemComponent.BP_ApplyGameplayEffectToSelf` _returnvalue (`self.Gameplay Effect Class`) 0.0 (`AbilitySystemComponent.MakeEffectContext` _returnvalue)))))))

(fn `UserConstructionScript`)