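; GA_SwapMode is a gameplay ability that toggles a player hero between Primary and Secondary mode.
; On activation it reads the owned gameplay tags from the ability system component on the avatar character's NDDPlayerState.
; If the Primary mode tag is present, it removes effects granting that tag and applies GE_SetMode_Secondary; otherwise it does the reverse.
; The ability then ends immediately, so the active gameplay effect carries the mode state.
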(event `self.K2_ActivateAbility`
  ;[0.6198 0.6198 0.6198 0.5] Get Owning PlayerState for grabbing Tags
  (bind _asnddcharacter (cast `NDDCharacter` (`self.GetAvatarActorFromActorInfo`)))
  (bind _asnddplayer_state (cast `NDDPlayerState` (`Pawn.PlayerState` _asnddcharacter)))
  ; Swap Primary Mode and Secondary Mode
  (if (`BlueprintGameplayTagLibrary.HasTag` (`BlueprintGameplayTagLibrary.GetOwnedGameplayTags` (`AbilitySystemBlueprintLibrary.GetAbilitySystemComponent` _asnddplayer_state)) (struct :`TagName` "State.Hero.PrimaryMode"))
    (`self.BP_RemoveGameplayEffectFromOwnerWithGrantedTags` (struct :`GameplayTags` (struct :`(TagName` "State.Hero.PrimaryMode"))))
    (`self.BP_ApplyGameplayEffectToOwner` "/Game/Networked_RPG/Characters/Players/GE_SetMode_Secondary.GE_SetMode_Secondary_C")
    (else
      (`self.BP_RemoveGameplayEffectFromOwnerWithGrantedTags` (struct :`GameplayTags` (struct :`(TagName` "State.Hero.SecondaryMode"))))
      (`self.BP_ApplyGameplayEffectToOwner` "/Game/Networked_RPG/Characters/Players/GE_SetMode_Primary.GE_SetMode_Primary_C")))
  (`self.K2_EndAbility`))